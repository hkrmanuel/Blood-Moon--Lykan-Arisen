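; Player-controlled Paper2D character with side-scrolling movement, jumping and a three-step attack chain, driven by Enhanced Input.
; Movement input plays the run flipbook and rotates the sprite to face the travel direction, but is ignored during jumps.
; Jumping polls vertical velocity with a Delay loop to detect landing.
; Flags advance successive attacks through three non-looping flipbooks, and finished playback restores looping idle.
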(event `self.ReceiveBeginPlay`
  (bind _asbp_player_controller (cast `/Game/Blueprints/Werewolf_Prints/BP_Player_controller` (`self.GetController`)))
  (`EnhancedInputSubsystemInterface.AddMappingContext` (pcsubsystem `EnhancedInputLocalPlayerSubsystem` _asbp_player_controller) "/Game/Blueprints/Werewolf_Prints/IMC_Default.IMC_Default" 0 (struct)))

(event `EnhancedInput|/Game/Blueprints/Werewolf_Prints/MOVEMENT`
  (params (ActionValue :type "Float (double-precision)") (ElapsedSeconds :type "Float (double-precision)") (TriggeredSeconds :type "Float (double-precision)") (InputAction :type "InputAction Object Reference" :default "/Game/Blueprints/Werewolf_Prints/MOVEMENT.MOVEMENT"))
  (:`Triggered`
    (if (not (`self.bls_jumping`))
      (`self.AddMovementInput` (`self.GetActorForwardVector`) ActionValue)
      (`PaperFlipbookComponent.SetFlipbook` (`self.Sprite`) "/Game/Assets6/Characters/Animations/Werewolf/Run1.Run1")
      (if (> ActionValue 0.0)
        (`SceneComponent.K2_SetWorldRotation` :`self` (`self.Sprite`))
        (else
          (`SceneComponent.K2_SetWorldRotation` (`self.Sprite`) (struct :`Yaw` -180.0) false false)))))
  (:`Completed`
    (if (not (`self.bls_jumping`))
      (`PaperFlipbookComponent.SetFlipbook` (`self.Sprite`) "/Game/Assets6/Characters/Animations/Werewolf/Idle1.Idle1"))))

(event `EnhancedInput|/Game/Blueprints/Werewolf_Prints/Jump`
  (params (ActionValue :type "Float (double-precision)") (ElapsedSeconds :type "Float (double-precision)") (TriggeredSeconds :type "Float (double-precision)") (InputAction :type "InputAction Object Reference" :default "/Game/Blueprints/Werewolf_Prints/Jump.Jump"))
  (bind _sprite (`self.Sprite`))
  (:`Triggered`
    (if (not (`self.bls_jumping`))
      (set `self.bls_jumping` true)
      (`self.Jump`)
      (`PaperFlipbookComponent.SetLooping` _sprite false)
      (`PaperFlipbookComponent.SetFlipbook` _sprite "/Game/Assets6/Characters/Animations/Werewolf/Jump1.Jump1")
      (`KismetSystemLibrary.Delay` 0.1)
      (if (== (.z (`self.GetVelocity`)) 0.0) :!label _label
        (`PaperFlipbookComponent.SetLooping` _sprite true)
        (`PaperFlipbookComponent.Play` _sprite)
        (`PaperFlipbookComponent.SetFlipbook` _sprite "/Game/Assets6/Characters/Animations/Werewolf/Idle1.Idle1")
        (set `self.bls_jumping` false)
        (else
          (`KismetSystemLibrary.Delay` 0.1)
          (goto _label))))))

(event `EnhancedInput|/Game/Blueprints/Werewolf_Prints/Attack`
  (params (ActionValue :type "Float (double-precision)") (ElapsedSeconds :type "Float (double-precision)") (TriggeredSeconds :type "Float (double-precision)") (InputAction :type "InputAction Object Reference" :default "/Game/Blueprints/Werewolf_Prints/Attack.Attack"))
  (:`Triggered`
    (if (`self.bls_attack2`)
      (`PaperFlipbookComponent.SetFlipbook` (`self.Sprite`) "/Game/Assets6/Characters/Animations/Werewolf/Attack2.Attack2")
      (`PaperFlipbookComponent.SetLooping` (`self.Sprite`) false)
      (set `self.bls_attack3` true)
      (set `self.bls_attack2` false)
      (elif (`self.bls_attack3`)
        (`PaperFlipbookComponent.SetFlipbook` (`self.Sprite`) "/Game/Assets6/Characters/Animations/Werewolf/Attack3.Attack3")
        (`PaperFlipbookComponent.SetLooping` (`self.Sprite`) false)
        (set `self.bls_attack3` false)
        (else
          (`PaperFlipbookComponent.SetFlipbook` (`self.Sprite`) "/Game/Assets6/Characters/Animations/Werewolf/Attack1.Attack1")
          (`PaperFlipbookComponent.SetLooping` (`self.Sprite`) false)
          (set `self.bls_attack2` true)
          (set `self.bls_attack` false))))))

(event `self.Sprite.OnFinishedPlaying`
  (`PaperFlipbookComponent.SetFlipbook` (`self.Sprite`) "/Game/Assets6/Characters/Animations/Werewolf/Idle1.Idle1")
  (`PaperFlipbookComponent.SetLooping` (`self.Sprite`) true)
  (if (not (`PaperFlipbookComponent.IsPlaying` (`self.Sprite`)))
    (`PaperFlipbookComponent.Play` (`self.Sprite`))))

(fn `UserConstructionScript`)